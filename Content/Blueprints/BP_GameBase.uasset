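; BP_GameBase holds the score state for a duel between a Demon King and a Hero, each with sword and shield values.
; Setters store those values and two fluctuation ranges, and GameFinish sets and returns Wining when the Devil's total lead reaches 65% of the summed ranges.
; BeginPlay forces 1080p, and Tick prints debug totals in Chinese, though the Devil's printed total adds its sword value twice, omitting the shield.
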(event `self.ReceiveBeginPlay`
  (`KismetSystemLibrary.ExecuteConsoleCommand` "r.setres 1920x1080" null))

(event `self.ReceiveTick`
  (params (DeltaSeconds :type "Float (single-precision)"))
  (`KismetSystemLibrary.PrintString` (`KismetStringLibrary.Concat_StrStr` (`KismetStringLibrary.Concat_StrStr` "剑的浮动范围值为" (`KismetStringLibrary.Conv_DoubleToString` (`self.X1`))) (`KismetStringLibrary.Concat_StrStr` "           盾的浮动范围为" (`KismetStringLibrary.Conv_DoubleToString` (`self.X2`)))))
  (`KismetSystemLibrary.PrintString` (`KismetStringLibrary.Concat_StrStr` (`KismetStringLibrary.Concat_StrStr` "魔王的力量值为：" (`KismetStringLibrary.Conv_DoubleToString` (+ (`self.DevilSwordValue`) (`self.DevilSwordValue`)))) (`KismetStringLibrary.Concat_StrStr` "勇者的力量值为：" (`KismetStringLibrary.Conv_DoubleToString` (+ (`self.PlayerSowrdValue`) (`self.PlayerShiledValue`)))))))

(fn `GameFinish`
  (returns (Win :type Boolean))
  (bind _returnvalue (>= (- (+ (`self.DevilSwordValue`) (`self.DevilShiledValue`)) (+ (`self.PlayerSowrdValue`) (`self.PlayerShiledValue`))) (* (+ (`self.X1`) (`self.X2`)) 0.65)))
  (set `self.bWining` _returnvalue)
  (return _returnvalue))

(fn `Set Condition`
  (params (X1 :type "Float (double-precision)") (X2 :type "Float (double-precision)"))
  (set `self.X1` X1)
  (set `self.X2` X2))

(fn `SetDevil`
  (params (DevilSwordValue :type "Float (double-precision)") (DevilShiledValue :type "Float (double-precision)"))
  (set `self.DevilSwordValue` DevilSwordValue)
  (set `self.DevilShiledValue` DevilShiledValue))

(fn `SetPlayerShiled`
  (params (ShiledValue :type "Float (double-precision)"))
  (set `self.PlayerShiledValue` ShiledValue))

(fn `SetPlayerSword`
  (params (SwordValue :type "Float (double-precision)"))
  (set `self.PlayerSowrdValue` SwordValue))

(fn `UserConstructionScript`)