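; Player controller that caches references to the controlled BP_Player and BP_GameInstance on BeginPlay.
; MoveCharacter passes a goal to SimpleMoveToLocation for navigation-based pawn movement, with no caller in this file.
; The MoveRight axis event is empty; its camera-relative AddMovementInput and debug print are left disconnected.
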(event `self.ReceiveBeginPlay`
  (bind _asbp_player (cast `/Game/Blueprints/BP_Player` (`self.K2_GetPawn`)))
  (set `self.As BP Player` _asbp_player)
  (bind _asbp_game_instance (cast `/Game/Blueprints/BP_GameInstance` (`GameplayStatics.GetGameInstance`)))
  (set `self.As BP Game Instance` _asbp_game_instance))

(event `InputAxis|MoveRight`
  (params (AxisValue :type "Float (single-precision)"))
  ;[1 1 1] 移动
)

(fn `MoveCharacter`
  (params (Goal :type "Vector Structure (by ref)"))
  (`AIBlueprintHelperLibrary.SimpleMoveToLocation` self Goal))

(fn `UserConstructionScript`)