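; BP_Floor is a floor actor with a two-leaf iron gate that opens and closes around the player.
; On BeginPlay and when the player enters Box, it passes its location to BP_Controller's MoveCharacter.
; A timeline rotates the gate leaves open after a delay on entry, and reverses after a shorter delay on exit.
; Leaving Box_Open on the positive-Y side also plays the timeline, clearing the OpenGate flag that guards it.
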(event `self.ReceiveBeginPlay`
  (bind _asbp_game_instance (cast `/Game/Blueprints/BP_GameInstance` (`GameplayStatics.GetGameInstance`)))
  (set `self.As BP Game Instance` _asbp_game_instance)
  (bind _asbp_controller (cast `/Game/Blueprints/BP_Controller` (`GameplayStatics.GetPlayerController` 0)))
  (`/Game/Blueprints/BP_Controller.MoveCharacter` _asbp_controller (`self.K2_GetActorLocation`)))

(event `self.Box.OnComponentBeginOverlap`
  (params (OverlappedComponent :type "PrimitiveComponent Object Reference") (OtherActor :type "Actor Object Reference") (OtherComp :type "PrimitiveComponent Object Reference") (OtherBodyIndex :type Integer) (bFromSweep :type Boolean) (SweepResult :type "HitResult Structure (by ref)"))
  (bind _asbp_controller (cast `/Game/Blueprints/BP_Controller` (`GameplayStatics.GetPlayerController` 0)))
  (cast `/Game/Blueprints/BP_Player` OtherActor)
  (bind _asbp_controller_2 (cast `/Game/Blueprints/BP_Controller` (`GameplayStatics.GetPlayerController` 0)))
  (`/Game/Blueprints/BP_Controller.MoveCharacter` _asbp_controller_2 (`self.K2_GetActorLocation`))
  (`KismetSystemLibrary.PrintString` "Player Hit floor")
  (`KismetSystemLibrary.Delay` 5.0)
  (bind (_direction _left_ _right_) (`Timeline|时间轴_0` :!via `PlayFromStart` :!label _label)
    (:`Update`
      (`SceneComponent.K2_SetRelativeRotation` (`self.SM_Bld_Castle_Iron_Gate_left`) (`KismetMathLibrary.MakeRotator` _left_) false false)
      (`SceneComponent.K2_SetRelativeRotation` (`self.SM_Bld_Castle_Iron_Gate_righ`) (`KismetMathLibrary.MakeRotator` _right_ 0.0 -180.0) false false))))

(event `self.Box.OnComponentEndOverlap`
  (params (OverlappedComponent :type "PrimitiveComponent Object Reference") (OtherActor :type "Actor Object Reference") (OtherComp :type "PrimitiveComponent Object Reference") (OtherBodyIndex :type Integer))
  (cast `/Game/Blueprints/BP_Player` OtherActor)
  (`KismetSystemLibrary.Delay` 1.0)
  (goto _label :!via `ReverseFromEnd`))

(event `self.Box_Open.OnComponentEndOverlap`
  (params (OverlappedComponent :type "PrimitiveComponent Object Reference") (OtherActor :type "Actor Object Reference") (OtherComp :type "PrimitiveComponent Object Reference") (OtherBodyIndex :type Integer))
  (if (`self.bOpenGate`)
    (bind _asbp_player (cast `/Game/Blueprints/BP_Player` OtherActor))
    (if (> (- (.y (`self.K2_GetActorLocation` _asbp_player)) (.y (`self.K2_GetActorLocation`))) 0.0)
      (set `self.bOpenGate` false)
      (goto _label :!via `PlayFromStart`))))

(fn `UserConstructionScript`)