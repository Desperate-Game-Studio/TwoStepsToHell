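; Trigger volume actor that controls the house background sound as the player enters and leaves its Box.
; BeginPlay creates the BG_House 2D sound component and stores it for reuse.
; On Box overlap with BP_Player, it plays the sound from the start and issues an AIMoveTo sending the player pawn to a hardcoded location.
; When BP_Player leaves the Box, it pauses the sound.
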(event `self.ReceiveBeginPlay`
  (bind _returnvalue (`GameplayStatics.CreateSound2D` "/Game/Sound/BG_House.BG_House" 1.0 1.0 0.0 null))
  (set `self.NewVar_0` _returnvalue))

(event `self.Box.OnComponentEndOverlap`
  (params (OverlappedComponent :type "PrimitiveComponent Object Reference") (OtherActor :type "Actor Object Reference") (OtherComp :type "PrimitiveComponent Object Reference") (OtherBodyIndex :type Integer))
  (cast `/Game/Blueprints/BP_Player` OtherActor)
  (`AudioComponent.SetPaused` (`self.NewVar_0`) true))

(event `self.Box.OnComponentBeginOverlap`
  (params (OverlappedComponent :type "PrimitiveComponent Object Reference") (OtherActor :type "Actor Object Reference") (OtherComp :type "PrimitiveComponent Object Reference") (OtherBodyIndex :type Integer) (bFromSweep :type Boolean) (SweepResult :type "HitResult Structure (by ref)"))
  (bind _asbp_player (cast `/Game/Blueprints/BP_Player` OtherActor))
  (`AudioComponent.Play` (`self.NewVar_0`) 0.0)
  (`|AIMoveTo` _asbp_player (-260.0 -1710.0 270.0) null 3.0))

(fn `UserConstructionScript`)