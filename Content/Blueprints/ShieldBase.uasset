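; ShieldBase is a shield pickup that attaches its SwordBody component to the player on contact.
; When BP_Player overlaps the Box, it snaps SwordBody to a mesh socket, prints a debug message, disables Box collision and applies the stored scale through SetSize.
; It passes the scale's Z as the shield value to BP_GameBase, then after a short delay teleports the player to a hardcoded location and removes all widgets.
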(event `self.Box.OnComponentBeginOverlap`
  (params (OverlappedComponent :type "PrimitiveComponent Object Reference") (OtherActor :type "Actor Object Reference") (OtherComp :type "PrimitiveComponent Object Reference") (OtherBodyIndex :type Integer) (bFromSweep :type Boolean) (SweepResult :type "HitResult Structure (by ref)"))
  (bind _value (`self.Value`))
  (bind _asbp_player (cast `/Game/Blueprints/BP_Player` OtherActor))
  (`SceneComponent.K2_AttachToComponent` (`self.SwordBody`) (`Character.Mesh` _asbp_player) (`self.Socket Name`) "SnapToTarget" "SnapToTarget" "SnapToTarget" false)
  (`KismetSystemLibrary.PrintString` "盾牌碰撞到角色" true true (struct :`R` 0.245106 :`G` 1.0 :`B` 0.310847 :`A` 1.0) 1.2)
  (`PrimitiveComponent.SetCollisionEnabled` (`self.Box`) "NoCollision")
  (`self.SetSize` _value)
  (bind _asbp_game_base (cast `/Game/Blueprints/BP_GameBase` (`GameplayStatics.GetGameMode`)))
  (`/Game/Blueprints/BP_GameBase.SetPlayerShiled` _asbp_game_base (.z _value))
  (`KismetSystemLibrary.Delay` 0.5)
  (`self.K2_SetActorLocation` _asbp_player (10.0 5480.0 230.0) false false)
  (`WidgetLayoutLibrary.RemoveAllWidgets`))

(fn `SetSize`
  (params (NewScale :type "Vector Structure"))
  (bind _output_get (set `self.Value` NewScale))
  (`SceneComponent.SetWorldScale3D` (`self.SwordBody`) _output_get))

(fn `UserConstructionScript`)