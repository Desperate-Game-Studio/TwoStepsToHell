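; Base weapon pickup that attaches itself to the player when a BP_Player overlaps its Box.
; On overlap, Body snaps to a socket on the player's mesh, a debug message prints and the Box collision is disabled.
; SetSize applies the stored world scale to Body, and the scale's Z is passed to BP_GameBase through SetPlayerSword.
; After a short delay, the player is moved to a hardcoded location.
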(event `self.ReceiveBeginPlay`
  (bind _asbp_game_instance (cast `/Game/Blueprints/BP_GameInstance` (`GameplayStatics.GetGameInstance`)))
  (set `self.As BP Game Instance` _asbp_game_instance))

(event `self.Box.OnComponentBeginOverlap`
  (params (OverlappedComponent :type "PrimitiveComponent Object Reference") (OtherActor :type "Actor Object Reference") (OtherComp :type "PrimitiveComponent Object Reference") (OtherBodyIndex :type Integer) (bFromSweep :type Boolean) (SweepResult :type "HitResult Structure (by ref)"))
  (bind _value (`self.Value`))
  (bind _asbp_player (cast `/Game/Blueprints/BP_Player` OtherActor))
  (`SceneComponent.K2_AttachToComponent` (`self.Body`) (`Character.Mesh` _asbp_player) (`self.Socket Name`) "SnapToTarget" "SnapToTarget" "SnapToTarget" false)
  (`KismetSystemLibrary.PrintString` "武器碰撞到角色" true true (struct :`R` 0.245106 :`G` 1.0 :`B` 0.310847 :`A` 1.0) 1.2)
  (`PrimitiveComponent.SetCollisionEnabled` (`self.Box`) "NoCollision")
  (`self.SetSize` _value)
  (bind _asbp_game_base (cast `/Game/Blueprints/BP_GameBase` (`GameplayStatics.GetGameMode`)))
  (`/Game/Blueprints/BP_GameBase.SetPlayerSword` _asbp_game_base (.z _value))
  (`KismetSystemLibrary.Delay` 0.3)
  (`self.K2_SetActorLocation` _asbp_player (-40.0 3590.0 -450.0) false false))

(fn `SetSize`
  (params (NewScale :type "Vector Structure"))
  (bind _output_get (set `self.Value` NewScale))
  (`SceneComponent.SetWorldScale3D` (`self.Body`) _output_get))

(fn `UserConstructionScript`)